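; Player controller that casts a debug line trace from the camera when the left mouse button is pressed.
; The trace runs from the camera manager's location along its forward vector for BlockDistance on the Visibility channel.
; It draws the ray for a set duration and prints the impact location on a hit, with no further action taken.
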(event EventBeginPlay)

(event Input|MouseEvents|LeftMouseButton
  (params (Key :type Key%20Structure :default "None"))
  (bind _playercameramanager (Variables|Default|GetPlayerCameraManager))
  (bind _returnvalue (Camera|GetCameraLocation _playercameramanager))
  (:Pressed
    (bind (_outhit _returnvalue_2) (Collision|LineTraceByChannel _returnvalue (+ _returnvalue (* (Math|Vector|GetForwardVector (Camera|GetCameraRotation _playercameramanager)) (Variables|Default|GetBlockDistance))) "TraceTypeQuery1" false 0 "ForDuration" true "(R=1.000000,G=0.000000,B=0.000000,A=1.000000)" "(R=0.000000,G=1.000000,B=0.000000,A=1.000000)" 1e+01))
    (if _returnvalue_2
      (Development|PrintString (Utilities|String|ToString(Vector) (.Location (Collision|BreakHitResult _outhit))) true true "(R=0.000000,G=0.660000,B=1.000000,A=1.000000)" 1e+01))))

(fn ConstructionScript)